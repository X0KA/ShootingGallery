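; CheetahGun is a weapon Blueprint that currently auto-fires pooled bullets from Tick as test logic.
; A DoOnce reset by a one-second Delay paces each shot, taking the next actor from BulletPool and casting it to CheetaBullet.
; A spline's first point serves as the spawn location, and the vector to its second point sets the fire direction.
; Trigger press and release events only print debug strings.
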(event `self.ReceiveTick`
  (params (DeltaSeconds :type "Float (single-precision)"))
  (bind _splinecomponent (`self.splineComponent`))
  ;[1 1 1] Testing
  (`/Engine/EditorBlueprintResources/StandardMacros.DoOnce` false :!label _label
    (:`Completed`
      (bind _returnvalue (`ActorPoolComponent.GetNextActor` (`self.BulletPool`)))
      (`self.K2_SetActorLocation` _returnvalue (`SplineComponent.GetLocationAtSplinePoint` (`self.splineComponent`) 0 "World") false false)
      (bind _ascheeta_bullet (cast `/Game/Blueprints/Projectiles/CheetaBullet` _returnvalue))
      (`/Game/Blueprints/Projectiles/CheetaBullet.Fire` _ascheeta_bullet (- (`SplineComponent.GetLocationAtSplinePoint` _splinecomponent 1 "World") (`SplineComponent.GetLocationAtSplinePoint` _splinecomponent 0 "World")) 5.0)
      (`KismetSystemLibrary.Delay` 1.0)
      (goto _label :!via `Reset`))))

(event `self.OnTriggerPressed`
  ;[1 1 1] INput
  (`KismetSystemLibrary.PrintString` "Trigger pressed"))

(event `self.OnTriggerReleased`
  ;[1 1 1] INput
  (`KismetSystemLibrary.PrintString` "trigger released"))

(fn `UserConstructionScript`)