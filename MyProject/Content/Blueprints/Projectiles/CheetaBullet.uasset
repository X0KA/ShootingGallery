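; CheetaBullet is a physics-driven projectile Blueprint built to be fired repeatedly.
; Fire clears the sphere's linear velocity, applies a mass-dependent impulse along the given direction scaled by speed, records the fire time and clears ToDisable.
; Tick sets ToDisable once LifeDuration has elapsed, flagging the bullet rather than destroying it, which suggests pooling by an external owner.
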(event `self.ReceiveTick`
  (params (DeltaSeconds :type "Float (single-precision)"))
  (if (not (`self.toDisable`))
    (set `self.toDisable` (> (- (`KismetSystemLibrary.GetGameTimeInSeconds`) (`self.fireTime`)) (`self.lifeDuration`)))))

(fn `Fire`
  (params (Direction :type "Vector Structure") (Speed :type "Float (double-precision)"))
  (`PrimitiveComponent.SetPhysicsLinearVelocity` (`self.Sphere`) (0.0 0.0 0.0) false "None")
  (`PrimitiveComponent.AddImpulse` (`self.Sphere`) (* Direction Speed) "None" false)
  (set `self.fireTime` (`KismetSystemLibrary.GetGameTimeInSeconds`))
  (set `self.toDisable` false))

(fn `UserConstructionScript`)